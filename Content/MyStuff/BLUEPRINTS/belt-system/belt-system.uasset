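; Conveyor belt actor that builds two-lane belts from a Jsonloader's belt paths and animates items along them.
; Construction stitches one spline per path from straight, left and right template splines, rotated and placed on the grid.
; It randomly fills evenly spaced lane slots with item child actors by belt fullness, using a shared empty component for gaps.
; Tick derives each item's position from game time, wrapping at the spline's end.
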(event EventTick
  (params (DeltaSeconds :type Float%20%28single-precision%29))
  (for _array_element (Variables|Default|Getbelt_splines)
    (bind (_item_1 _item_2 _index) (Utilities|ForEachLoop(zip) (.lane_1_items (Utilities|Struct|BreakBeltSpline _array_element)) (.lane_2_items (Utilities|Struct|BreakBeltSpline _array_element)))
      (:Loop%20body
        (Transformation|SetWorldLocation _item_1 (.Location (Math|Transform|BreakTransform (Math|Transform|ComposeTransforms (Math|Transform|MakeTransform (Math|Vector|MakeVector 0.0 (Variables|Default|Getlane_spacing) 0.0)) (Spline|GetTransformatDistanceAlongSpline (.spline (Utilities|Struct|BreakBeltSpline _array_element)) (|((({A0475781-4F07-BC5B-B66F-03936B73FBE8}*index)+(game_time*{2F38E8AA-430D-0A9E-15D7-828A9188237F}))%spline_length) (Utilities|Time|GetGameTimeinSeconds) (Spline|GetSplineLength (.spline (Utilities|Struct|BreakBeltSpline _array_element))) _index) "World" false)))) false true)
        (Transformation|SetWorldLocation _item_2 (.Location (Math|Transform|BreakTransform (Math|Transform|ComposeTransforms (Math|Transform|MakeTransform (Math|Vector|MakeVector 0.0 (* (Variables|Default|Getlane_spacing) -1.0) 0.0)) (Spline|GetTransformatDistanceAlongSpline (.spline (Utilities|Struct|BreakBeltSpline _array_element)) (|((({A0475781-4F07-BC5B-B66F-03936B73FBE8}*index)+(game_time*{2F38E8AA-430D-0A9E-15D7-828A9188237F}))%spline_length) (Utilities|Time|GetGameTimeinSeconds) (Spline|GetSplineLength (.spline (Utilities|Struct|BreakBeltSpline _array_element))) _index) "World" false)))) false true)))))

(fn ConstructionScript
  (Variables|Default|Setbelt-splines-map (Utilities|Map|MakeMap "I" (Variables|Default|Getbelt-I_spline) "L" (Variables|Default|Getbelt-L_spline) "R" (Variables|Default|Getbelt-R_spline)))
  (bind _returnvalue (AddComponent|AddChildActorComponent false))
  (Variables|Default|SetemptyComponent _returnvalue)
  (bind _outactors (Actor|GetAllActorsOfClass "/Game/MyStuff/BLUEPRINTS/json-loader/json-loader.json-loader_C"))
  (for _array_element (Variables|/Game/MyStuff/BLUEPRINTS/json-loader/json-loader.json-loader_C|Getbelt-paths (Utilities|Array|Get(acopy) _outactors))
    (bind _returnvalue_2 (AddComponent|AddSplineComponent false))
    (Spline|ClearSplinePoints _returnvalue_2 true)
    (bind (_item_1 _item_2 _index_1) (Utilities|ForEachPairwise (.entities (Utilities|Struct|BreakBeltPath _array_element)))
      (:Loop%20body
        ;[1 1 1] Create belt spline
        (bind (_position _tangent) (CallFunction|GetSplinePoint _item_1 false))
        (bind (_position_2 _tangent_2) (CallFunction|GetSplinePoint _item_2 true))
        (Spline|AddSplinePoint _returnvalue_2 (Math|Vector|SelectVector _position _position_2 (>= _index_1 0)) "Local" true)
        (Spline|SetTangentsatSplinePoint _returnvalue_2 (- (Spline|GetNumberOfSplinePoints _returnvalue_2) 1) _tangent _tangent_2 "Local" true))
      (:Completed
        ;[1 1 1] Spawn items on belts
        (bind _arrayout (Utilities|SetTempArray (Utilities|Array|MakeArray))
          (:ExecOut
            (bind _arrayout_2 (Utilities|SetTempArray (Utilities|Array|MakeArray))
              (:ExecOut
                (for _index (range 0 (|(floor((splineLength/{A0475781-4F07-BC5B-B66F-03936B73FBE8}))) (Spline|GetSplineLength _returnvalue_2)))
                  (if (|((arrayLength>0)&&(((random())*100)<={8CB7980C-4544-68F2-14C6-9A81CBFF529E})) (Utilities|Array|Length (.right_lane_items (Utilities|Struct|BreakBeltPath _array_element))))
                    (bind _returnvalue_3 (AddComponent|AddChildActorComponent false (Math|Transform|MakeTransform (.Location (Math|Transform|BreakTransform (Math|Transform|ComposeTransforms (Math|Transform|MakeTransform (Math|Vector|MakeVector 0.0 (Variables|Default|Getlane_spacing) 0.0)) (Spline|GetTransformatDistanceAlongSpline _returnvalue_2 (|(index*{A0475781-4F07-BC5B-B66F-03936B73FBE8}) _index) "Local" false)))) "0.000000,0.000000,4.000000")))
                    (ChildActorComponent|SetChildActorClass _returnvalue_3 (.Value (Utilities|Map|Find (Variables|Default|Getitem-list) (.OutItem (Utilities|Array|Random (.right_lane_items (Utilities|Struct|BreakBeltPath _array_element)))))))
                    (Utilities|Array|Add _arrayout _returnvalue_3)
                    (else
                      (Utilities|Array|Add _arrayout (Variables|Default|GetemptyComponent))))
                  (if (|((arrayLength>0)&&(((random())*100)<={8CB7980C-4544-68F2-14C6-9A81CBFF529E})) (Utilities|Array|Length (.left_lane_items (Utilities|Struct|BreakBeltPath _array_element))))
                    (bind _returnvalue_4 (AddComponent|AddChildActorComponent false (Math|Transform|MakeTransform (.Location (Math|Transform|BreakTransform (Math|Transform|ComposeTransforms (Math|Transform|MakeTransform (Math|Vector|MakeVector 0.0 (* (Variables|Default|Getlane_spacing) -1.0) 0.0)) (Spline|GetTransformatDistanceAlongSpline _returnvalue_2 (|(index*{A0475781-4F07-BC5B-B66F-03936B73FBE8}) _index) "Local" false)))) "0.000000,0.000000,4.000000")))
                    (ChildActorComponent|SetChildActorClass _returnvalue_4 (.Value (Utilities|Map|Find (Variables|Default|Getitem-list) (.OutItem (Utilities|Array|Random (.left_lane_items (Utilities|Struct|BreakBeltPath _array_element)))))))
                    (Utilities|Array|Add _arrayout_2 _returnvalue_4)
                    (else
                      (Utilities|Array|Add _arrayout_2 (Variables|Default|GetemptyComponent)))))
                (Utilities|Array|Add (Variables|Default|Getbelt_splines) (Utilities|Struct|MakeBeltSpline _returnvalue_2 _arrayout _arrayout_2))))))))))

(fn GetSplinePoint
  (params (Belt :type Exported%20Entity%20Structure%20%28by%20ref%29) (GetSplineStartPoint :type Boolean))
  (bind (_x _y _direction _variant) (Utilities|Struct|BreakExportedEntity Belt))
  (bind _belt_splines_map (Variables|Default|Getbelt-splines-map))
  (bind _value (Utilities|Map|Find _belt_splines_map _variant))
  (bind _returnvalue (|(direction*45.000000) _direction))
  (bind _returnvalue_2 (Math|Rotator|MakeRotator 0.0 0.0 _returnvalue))
  (return (+ (Math|Vector|RotateVector (Spline|GetLocationatSplinePoint _value (Math|Integer|SelectInt 0 1 GetSplineStartPoint) "Local") _returnvalue_2) (* (Math|Vector|MakeVector _x _y 0.0) "200.000000,200.000000,0.000000")) (Math|Vector|RotateVector (Math|Vector|SelectVector (Spline|GetLeaveTangentatSplinePoint _value 0 "Local") (Spline|GetArriveTangentatSplinePoint _value 1 "Local") GetSplineStartPoint) _returnvalue_2)))