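; JSON loader actor that rebuilds an exported factory layout (entities, wires, train and belt paths, logistic networks) in the level.
; Its construction script reads a chosen file, or a default project JSON, and parses each section into struct arrays.
; Entities load first because paths and logistic systems reference them by index.
; It then adds base spawner and belt system child actors; rail and logistic spawners are disconnected.
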(event EventBeginPlay)

(event Collision|EventActorBeginOverlap
  (params (OtherActor :type Actor%20Object%20Reference)))

(event EventTick
  (params (DeltaSeconds :type Float%20%28single-precision%29)))

(fn ConstructionScript
  (bind _filepath (Variables|Default|Getfilepath))
  (bind _outjsonobject (Class|JsonBlueprintFunctionLibrary|FromFile (Utilities|Struct|MakeFilePath (Utilities|String|SelectString (Class|BlueprintPathsLibrary|Combine (Utilities|Array|MakeArray (Class|KismetSystemLibrary|GetProjectDirectory) "Content" "MyStuff" "JSON" "exported-entities.json")) _filepath (Utilities|Array|IsEmpty _filepath)))))
  (Utilities|FlowControl|Sequence
    (:then_0
      ;[1 1 1] Load JSON
      (bind _outvalue (|GetJsonField _outjsonobject "entities"))
      (for _array_element _outvalue
        (bind _result (CallFunction|ParseExportedEntity _array_element))
        (Utilities|Array|Add (Variables|Default|Getexported-entities) _result)))
    (:then_1
      (bind _outvalue_2 (|GetJsonField _outjsonobject "wire_connections"))
      (for _array_element_2 _outvalue_2
        (bind _result_2 (CallFunction|ParseWireConnection _array_element_2))
        (Utilities|Array|Add (Variables|Default|Getwire-connections) _result_2)))
    (:then_2
      (bind _outvalue_3 (|GetJsonField _outjsonobject "train_paths"))
      (for _array_element_3 _outvalue_3
        (bind _result_3 (CallFunction|ParseTrainPath _array_element_3))
        (Utilities|Array|Add (Variables|Default|Gettrain-paths) _result_3)))
    (:then_3
      (bind _outvalue_4 (|GetJsonField _outjsonobject "belt_paths"))
      (for _array_element_4 _outvalue_4
        (bind _result_4 (CallFunction|ParseBeltPath _array_element_4))
        (Utilities|Array|Add (Variables|Default|Getbelt-paths) _result_4)))
    (:then_4
      (bind _outvalue_5 (|GetJsonField _outjsonobject "logistic_systems"))
      (for _array_element_5 _outvalue_5
        (bind _result_5 (CallFunction|ParseLogisticSystem _array_element_5))
        (Utilities|Array|Add (Variables|Default|Getlogistic-systems) _result_5)))
    (:then_5
      ;[1 1 1] Spawn systems
      (Utilities|FlowControl|Sequence
        (:then_0
          (bind _returnvalue (AddComponent|AddChildActorComponent false))
          (ChildActorComponent|SetChildActorClass _returnvalue "/Game/MyStuff/BLUEPRINTS/base-spawner/base-spawner.base-spawner_C"))
        (:then_2
          (bind _returnvalue_2 (AddComponent|AddChildActorComponent false))
          (ChildActorComponent|SetChildActorClass _returnvalue_2 "/Game/MyStuff/BLUEPRINTS/belt-system/belt-system.belt-system_C"))))))

(fn ParseExportedEntity
  (params (JsonObject :type Json%20Object%20Wrapper%20Structure%20%28by%20ref%29))
  (bind _outvalue (|GetJsonField JsonObject "name"))
  (bind _outvalue_2 (|GetJsonField JsonObject "x"))
  (bind _outvalue_3 (|GetJsonField JsonObject "y"))
  (bind _outvalue_4 (|GetJsonField JsonObject "direction"))
  (bind _outvalue_5 (|GetJsonField JsonObject "width"))
  (bind _outvalue_6 (|GetJsonField JsonObject "height"))
  (bind _outvalue_7 (|GetJsonField JsonObject "back_mover"))
  (bind _outvalue_8 (|GetJsonField JsonObject "operation"))
  (bind _outvalue_9 (|GetJsonField JsonObject "variant"))
  (return (Utilities|Struct|MakeExportedEntity _outvalue _outvalue_2 _outvalue_3 _outvalue_4 _outvalue_5 _outvalue_6 _outvalue_7 _outvalue_8 _outvalue_9)))

(fn ParseWireConnection
  (params (JsonObject :type Json%20Object%20Wrapper%20Structure%20%28by%20ref%29))
  (Utilities|FlowControl|Sequence
    (:then_0
      (bind _outvalue (|GetJsonField JsonObject "start"))
      (bind _outvalue_2 (|GetJsonField _outvalue "x"))
      (bind _outvalue_3 (|GetJsonField _outvalue "y"))
      (bind _outvalue_4 (|GetJsonField _outvalue "z")))
    (:then_1
      (bind _outvalue_5 (|GetJsonField JsonObject "target"))
      (bind _outvalue_6 (|GetJsonField _outvalue_5 "x"))
      (bind _outvalue_7 (|GetJsonField _outvalue_5 "y"))
      (bind _outvalue_8 (|GetJsonField _outvalue_5 "z")))
    (:then_2
      (return (Utilities|Struct|MakeWireConnection (Math|Vector|MakeVector _outvalue_2 _outvalue_3 _outvalue_4) (Math|Vector|MakeVector _outvalue_6 _outvalue_7 _outvalue_8))))))

(fn ParseTrainPath
  (params (JsonObject :type Json%20Object%20Wrapper%20Structure%20%28by%20ref%29))
  (Utilities|FlowControl|Sequence
    (:then_0
      (bind _outvalue (|GetJsonField JsonObject "carriages"))
      (bind _arrayout (Utilities|SetTempArray (Utilities|Array|MakeArray))
        (:ExecOut
          (for _array_element _outvalue
            (Utilities|Array|Add _arrayout (Utilities|Array|Get(acopy) (Variables|Default|Getexported-entities) _array_element))))))
    (:then_1
      (bind _outvalue_2 (|GetJsonField JsonObject "path"))
      (bind _arrayout_2 (Utilities|SetTempArray (Utilities|Array|MakeArray))
        (:ExecOut
          (for _array_element_2 _outvalue_2
            (bind _outvalue_3 (|GetJsonField _array_element_2 "index"))
            (bind _outvalue_4 (|GetJsonField _array_element_2 "invert_spline"))
            (Utilities|Array|Add _arrayout_2 (Utilities|Struct|MakeTrainPathSegment (Utilities|Array|Get(acopy) (Variables|Default|Getexported-entities) _outvalue_3) _outvalue_4))))))
    (:then_2
      (return (Utilities|Struct|MakeTrainPath _arrayout _arrayout_2)))))

(fn ParseBeltPath
  (params (JsonObject :type Json%20Object%20Wrapper%20Structure%20%28by%20ref%29))
  (Utilities|FlowControl|Sequence
    (:then_0
      (bind _outvalue (|GetJsonField JsonObject "path"))
      (bind _arrayout (Utilities|SetTempArray (Utilities|Array|MakeArray))
        (:ExecOut
          (for _array_element _outvalue
            (Utilities|Array|Add _arrayout (Utilities|Array|Get(acopy) (Variables|Default|Getexported-entities) _array_element))))))
    (:then_1
      (bind _outvalue_2 (|GetJsonField JsonObject "items_lane_1"))
      (bind _arrayout_2 (Utilities|SetTempArray (Utilities|Array|MakeArray))
        (:ExecOut
          (for _array_element_2 _outvalue_2
            (Utilities|Array|Add _arrayout_2 _array_element_2)))))
    (:then_2
      (bind _outvalue_3 (|GetJsonField JsonObject "items_lane_2"))
      (bind _arrayout_3 (Utilities|SetTempArray (Utilities|Array|MakeArray))
        (:ExecOut
          (for _array_element_3 _outvalue_3
            (Utilities|Array|Add _arrayout_3 _array_element_3)))))
    (:then_3
      (return (Utilities|Struct|MakeBeltPath _arrayout _arrayout_2 _arrayout_3)))))

(fn ParseLogisticSystem
  (params (JsonObject :type Json%20Object%20Wrapper%20Structure))
  (Utilities|FlowControl|Sequence
    (:then_0
      (bind _outvalue (|GetJsonField JsonObject "roboports"))
      (bind _arrayout (Utilities|SetTempArray (Utilities|Array|MakeArray))
        (:ExecOut
          (for _array_element _outvalue
            (Utilities|Array|Add _arrayout (Utilities|Array|Get(acopy) (Variables|Default|Getexported-entities) _array_element))))))
    (:then_1
      (bind _outvalue_2 (|GetJsonField JsonObject "chests"))
      (bind _arrayout_2 (Utilities|SetTempArray (Utilities|Array|MakeArray))
        (:ExecOut
          (for _array_element_2 _outvalue_2
            (Utilities|Array|Add _arrayout_2 (Utilities|Array|Get(acopy) (Variables|Default|Getexported-entities) _array_element_2))))))
    (:then_2
      (return (Utilities|Struct|MakeLogisticSystem _arrayout _arrayout_2)))))