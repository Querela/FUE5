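; Base spawner actor that builds a grid-based base layout in its Construction Script from the first Jsonloader's exported entities and wire connections.
; Each entity name is looked up in category maps to spawn a placed, rotated child actor with its variant set, while Missing entries become scaled cubes.
; Wires are child actors aimed and stretched between endpoints.
; Maximum entity coordinates size the Landscape and a tiled ground mesh.
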(fn ConstructionScript
  (bind _returnvalue (Math|Float|MakeLiteralFloat 0.12))
  (bind _static (Variables|Default|Getstatic))
  (bind _outactors (Actor|GetAllActorsOfClass "/Game/MyStuff/BLUEPRINTS/json-loader/json-loader.json-loader_C"))
  (Utilities|FlowControl|Sequence
    (:then_0
      ;[1 1 1] Spawn entities
      (for _array_element (Variables|/Game/MyStuff/BLUEPRINTS/json-loader/json-loader.json-loader_C|Getexported-entities (Utilities|Array|Get(acopy) _outactors))
        ;;[1 1 1] choose entity and spawn
        (bind _returnvalue_2 (AddComponent|AddChildActorComponent false (Math|Transform|MakeTransform (* (Math|Vector|MakeVector (.x (Utilities|Struct|BreakExportedEntity _array_element)) (.y (Utilities|Struct|BreakExportedEntity _array_element)) 0.0) "200.000000,200.000000,200.000000") (* (Math|Rotator|MakeRotator 0.0 0.0 (Math|Conversions|ToFloat(Integer) (.direction (Utilities|Struct|BreakExportedEntity _array_element)))) 45.0))))
        (if (.ReturnValue (Utilities|Map|Find (Variables|Default|Getvariants) (.name (Utilities|Struct|BreakExportedEntity _array_element))))
          (ChildActorComponent|SetChildActorClass _returnvalue_2 (.Value (Utilities|Map|Find (Variables|Default|Getvariants) (.name (Utilities|Struct|BreakExportedEntity _array_element)))))
          (bind _as_has_variants (Utilities|Casting|CastTo_HasVariants (Variables|/Script/Engine.ChildActorComponent|GetChildActor _returnvalue_2) :!label _label)
            (:then
              (Default|SetVariant _as_has_variants (.variant (Utilities|Struct|BreakExportedEntity _array_element))))
            (:CastFailed
              _))
          (Utilities|Struct|SetmembersinExportedEntity _array_element (Variables|/Script/Engine.ChildActorComponent|GetChildActor _returnvalue_2) :!label _label_2)
          (elif (.ReturnValue (Utilities|Map|Find (Variables|Default|Getstructures) (.name (Utilities|Struct|BreakExportedEntity _array_element))))
            (ChildActorComponent|SetChildActorClass _returnvalue_2 (.Value (Utilities|Map|Find (Variables|Default|Getstructures) (.name (Utilities|Struct|BreakExportedEntity _array_element)))))
            (goto _label)
            (elif (.ReturnValue (Utilities|Map|Find (Variables|Default|Getpower) (.name (Utilities|Struct|BreakExportedEntity _array_element))))
              (ChildActorComponent|SetChildActorClass _returnvalue_2 (.Value (Utilities|Map|Find (Variables|Default|Getpower) (.name (Utilities|Struct|BreakExportedEntity _array_element)))))
              (goto _label)
              (elif (.ReturnValue (Utilities|Map|Find (Variables|Default|Getfoliage) (.name (Utilities|Struct|BreakExportedEntity _array_element))))
                (ChildActorComponent|SetChildActorClass _returnvalue_2 (.Value (Utilities|Map|Find (Variables|Default|Getfoliage) (.name (Utilities|Struct|BreakExportedEntity _array_element)))))
                (goto _label)
                (elif (.ReturnValue (Utilities|Map|Find (Variables|Default|Getmissing) (.name (Utilities|Struct|BreakExportedEntity _array_element))))
                  (bind _returnvalue_3 (AddComponent|AddStaticMeshComponent false (Math|Transform|MakeTransform (* (Math|Vector|MakeVector (.x (Utilities|Struct|BreakExportedEntity _array_element)) (.y (Utilities|Struct|BreakExportedEntity _array_element)) 0.0) "200.000000,200.000000,200.000000") (* (Math|Rotator|MakeRotator 0.0 0.0 (Math|Conversions|ToFloat(Integer) (.direction (Utilities|Struct|BreakExportedEntity _array_element)))) 45.0) (* (Math|Vector|MakeVector (.width (Utilities|Struct|BreakExportedEntity _array_element)) (.height (Utilities|Struct|BreakExportedEntity _array_element)) 1.0) "2.000000,2.000000,2.000000"))))
                  (Components|StaticMesh|SetStaticMesh _returnvalue_3 "/Game/StarterContent/Shapes/Shape_Cube.Shape_Cube")
                  (goto _label_2))))))))
    (:then_1
      ;[1 1 1] wires
      (for _array_element_2 (Variables|/Game/MyStuff/BLUEPRINTS/json-loader/json-loader.json-loader_C|Getwire-connections (Utilities|Array|Get(acopy) _outactors))
        (bind _returnvalue_4 (AddComponent|AddChildActorComponent false (Math|Conversions|ToTransform(Vector) (* (.start (Utilities|Struct|BreakWireConnection _array_element_2)) "200.000000,200.000000,200.000000"))))
        (Transformation|SetRelativeRotation _returnvalue_4 (Math|Rotator|FindLookatRotation (* (.start (Utilities|Struct|BreakWireConnection _array_element_2)) "200.000000,200.000000,200.000000") (* (.target (Utilities|Struct|BreakWireConnection _array_element_2)) "200.000000,200.000000,200.000000")) false false)
        (Transformation|SetWorldScale3D _returnvalue_4 (Math|Vector|MakeVector (/ (Math|Vector|VectorLength (- (* (.start (Utilities|Struct|BreakWireConnection _array_element_2)) "200.000000,200.000000,200.000000") (* (.target (Utilities|Struct|BreakWireConnection _array_element_2)) "200.000000,200.000000,200.000000"))) 4e+02) 1.0 1.0))))
    (:then_2
      ;[1 1 1] Ground spawner
      (for _array_element_3 (Variables|/Game/MyStuff/BLUEPRINTS/json-loader/json-loader.json-loader_C|Getexported-entities (Utilities|Array|Get(acopy) _outactors))
        ;;[1 1 1] Find max
        (Variables|Default|SetmaxX (Math|Float|Max(Float) (.x (Utilities|Struct|BreakExportedEntity _array_element_3)) (Variables|Default|GetmaxX)))
        (Variables|Default|SetmaxY (Math|Float|Max(Float) (.y (Utilities|Struct|BreakExportedEntity _array_element_3)) (Variables|Default|GetmaxY))))
      ;;[1 1 1] landscape scale
      (bind _outactors_2 (Actor|GetAllActorsOfClass "/Script/Landscape.Landscape"))
      (Transformation|SetActorScale3D (Utilities|Array|Get(acopy) _outactors_2) (|(vector(({6A847684-4E42-93A1-2438-3BA3B5BD3896}*mul),({3196CA57-41E8-4013-E76C-018F76E9AC44}*mul),1)) 3.573))
      ;;[1 1 1] make plane
      (bind _returnvalue_5 (Rendering|Material|CreateDynamicMaterialInstance (Variables|Default|Getground-material) "" "None" :!class /Script/Engine.KismetMaterialLibrary))
      (Rendering|Material|SetScalarParameterValue _returnvalue_5 "UTiling" (* (Variables|Default|GetmaxX) _returnvalue) :!class /Script/Engine.MaterialInstanceDynamic)
      (Rendering|Material|SetScalarParameterValue _returnvalue_5 "VTiling" (* (Variables|Default|GetmaxY) _returnvalue) :!class /Script/Engine.MaterialInstanceDynamic)
      (Rendering|Material|SetMaterial _static 0 _returnvalue_5)
      (Transformation|SetRelativeScale3D _static (|(vector(({6A847684-4E42-93A1-2438-3BA3B5BD3896}*mul),({3196CA57-41E8-4013-E76C-018F76E9AC44}*mul),1)) 1.0)))))